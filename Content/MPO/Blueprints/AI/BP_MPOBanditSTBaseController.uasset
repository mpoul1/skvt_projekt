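; Base AI controller for MPO bandit enemies that relays player-sensing changes to a StateTree.
; PlayerSensedChanged turns the new sensed flag into a tagged StateTree event, EnemySense.PlayerSensed or EnemySense.PlayerLost, sent through the StateTreeAI component.
; BeginPlay and Tick are empty, and an unwired copy of the same branch, keyed on SuccessfullySensed, never runs.
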(event `self.ReceiveBeginPlay`)

(fn `PlayerSensedChanged`
  (params (NewPlayerSensed :type Boolean))
  (if NewPlayerSensed
    (`StateTreeComponent.SendStateTreeEvent` (`self.StateTreeAI`) (make `StateTreeEvent` (struct :`TagName` "EnemySense.PlayerSensed")))
    (else
      (`StateTreeComponent.SendStateTreeEvent` (`self.StateTreeAI`) (make `StateTreeEvent` (struct :`TagName` "EnemySense.PlayerLost"))))))

(fn `UserConstructionScript`)