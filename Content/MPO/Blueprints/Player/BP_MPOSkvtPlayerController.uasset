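; Player controller that lets the player cycle possession between BP_SkvtBaseChar characters in the level and toggle crouch on the controlled one.
; On BeginPlay it adds swap, crouch and default Enhanced Input mapping contexts at different priorities.
; Swap gathers all base characters, possesses the one after the current pawn with index wraparound, and prints its name.
; Crouch switches the controlled character between Crouch and UnCrouch.
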(event `self.ReceiveBeginPlay`
  (bind _returnvalue (pcsubsystem `EnhancedInputLocalPlayerSubsystem` self))
  ; Start Game - Assign Mapping Context
  (`/Engine/EditorBlueprintResources/StandardMacros.IsValid` _returnvalue
    (:`Is Valid`
      (`EnhancedInputSubsystemInterface.AddMappingContext` _returnvalue "/Game/MPO/PlayerController/IMC_MPOSwapPawn.IMC_MPOSwapPawn" 10 (struct))
      (`EnhancedInputSubsystemInterface.AddMappingContext` _returnvalue "/Game/MPO/PlayerController/IMC_MPOCrouchPawn.IMC_MPOCrouchPawn" 2 (struct))
      (`EnhancedInputSubsystemInterface.AddMappingContext` _returnvalue "/Game/Skvt/Input/IMC_Default.IMC_Default" 0 (struct)))))

(event `EnhancedInput|/Game/MPO/PlayerController/IA_MPOSwap`
  (params (ActionValue :type Boolean) (ElapsedSeconds :type "Float (double-precision)") (TriggeredSeconds :type "Float (double-precision)") (InputAction :type "InputAction Object Reference" :default "/Game/MPO/PlayerController/IA_MPOSwap.IA_MPOSwap"))
  ; Swap - Posses next available character in the scene
  (:`Triggered`
    (bind _outactors (`GameplayStatics.GetAllActorsOfClass` "/Game/Skvt/Characters/BP_SkvtBaseChar.BP_SkvtBaseChar_C"))
    (bind _foundcharacter (`self.FindNextCharacter` _outactors))
    (`self.Possess` _foundcharacter)
    (`KismetSystemLibrary.PrintString` (`KismetSystemLibrary.GetDisplayName` _foundcharacter))))

(event `EnhancedInput|/Game/MPO/PlayerController/IA_MPOCrouch`
  (params (ActionValue :type Boolean) (ElapsedSeconds :type "Float (double-precision)") (TriggeredSeconds :type "Float (double-precision)") (InputAction :type "InputAction Object Reference" :default "/Game/MPO/PlayerController/IA_MPOCrouch.IA_MPOCrouch"))
  ; Crouch
  (:`Triggered`
    (`self.ToggleCrouch` (`self.GetCurrectCharacter`))))

(fn `FindNextCharacter`
  (params (AllCharacters :type "Array of /Game/Skvt/Characters/BP_SkvtBaseChar Object Reference"))
  (returns (FoundCharacter :type "/Game/Skvt/Characters/BP_SkvtBaseChar Object Reference"))
  (bind _returnvalue (+ (`self.nextCharacterIndex`) 1))
  (set `self.allCharacters` AllCharacters)
  ; Find Current Character Index
  (bind _asbp_skvt_base_char (cast `/Game/Skvt/Characters/BP_SkvtBaseChar` (`self.K2_GetPawn`))
    (:`then`
      (bind _output_get (set `self.nextCharacterIndex` (`KismetArrayLibrary.Array_Find` (`self.allCharacters`) _asbp_skvt_base_char)))
      (if (< _output_get 0)
        (set `self.foundCharacter` null)
        (else
          ; Increment Character Index or Reset to 0
          (if (>= _returnvalue (`KismetArrayLibrary.Array_Length` (`self.allCharacters`)))
            (set `self.nextCharacterIndex` 0)
            (else
              (set `self.nextCharacterIndex` _returnvalue)))
          ; NextCharacterIndex to found Character
          (set `self.foundCharacter` (`|GetArrayItem` (`self.allCharacters`) (`self.nextCharacterIndex`))))))
    (:`CastFailed`
      _))
  (return (`self.foundCharacter`)))

(fn `GetCurrectCharacter`
  (returns (SkvtBaseCharacter :type "/Game/Skvt/Characters/BP_SkvtBaseChar Object Reference"))
  (bind _asbp_skvt_base_char (cast `/Game/Skvt/Characters/BP_SkvtBaseChar` (`self.K2_GetPawn`))
    (:`then`
      _)
    (:`CastFailed`
      _))
  (return _asbp_skvt_base_char))

(fn `ToggleCrouch`
  (params (characterToToggle :type "/Game/Skvt/Characters/BP_SkvtBaseChar Object Reference"))
  (returns (isCrouched :type Boolean) (canCrouch :type Boolean))
  (bind _biscrouched (`Character.bIsCrouched` characterToToggle))
  (if _biscrouched
    (`Character.UnCrouch` characterToToggle)
    (else
      (`Character.Crouch` characterToToggle)))
  (return (not _biscrouched) (`Character.CanCrouch` characterToToggle)))

(fn `UserConstructionScript`)